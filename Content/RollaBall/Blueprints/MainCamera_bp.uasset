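; MainCamera_bp is the Roll-a-Ball camera actor, which follows the player ball and displays its score.
; On BeginPlay it takes the first RollaBallPawn found in the level and stores its own starting location as an offset.
; Each Tick it writes the player's Score to a TextRender and moves to the player's location plus that offset, with no smoothing or sweep.
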(event `self.ReceiveBeginPlay`
  ;[1 1 1] Get player
  (bind _outactors (`GameplayStatics.GetAllActorsOfClass` "/Game/RollaBall/Blueprints/RollaBallPawn.RollaBallPawn_C"))
  (set `self.Player` (`|GetArrayItem` _outactors))
  ;[1 1 1] Store Starting Pos
  (set `self.OriginPos` (`self.K2_GetActorLocation`)))

(event `self.ReceiveTick`
  (params (DeltaSeconds :type "Float (single-precision)"))
  ;[1 1 1] Display Score
  (`TextRenderComponent.K2_SetText` (`self.TextRender`) (`KismetTextLibrary.Conv_IntToText` (`/Game/RollaBall/Blueprints/RollaBallPawn.Score` (`self.Player`))))
  ;[1 1 1] Add Camera Offset
  (`self.K2_SetActorLocation` (+ (`self.OriginPos`) (`self.K2_GetActorLocation` (`self.Player`)))))

(fn `UserConstructionScript`)